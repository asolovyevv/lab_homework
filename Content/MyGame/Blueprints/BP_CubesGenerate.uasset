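; BP_CubesGenerate is a placeable generator that spawns an X by Y grid of BP_Cube_Child actors spaced by Padding.
; The construction script builds an editor preview of the grid from static mesh components.
; BeginPlay destroys those previews, spawns the cubes at offsets from the actor's location and stores them in CubesArray.
; GetCubesForWin returns the array's length, apparently as the cube count needed to win.
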(event `self.ReceiveBeginPlay`
  (bind (_returnvalue_x _returnvalue_y _returnvalue_z) (`KismetMathLibrary.BreakVector` (`self.K2_GetActorLocation`)))
  (for _array_element (`self.PreviewArray`)
    (`ActorComponent.K2_DestroyComponent` _array_element))
  (for _index (range 1 (+ (`self.X`) 1))
    (for _index_2 (range 1 (+ (`self.Y`) 1))
      (bind _returnvalue (`|SpawnActorFromClass` "/Game/MyGame/Blueprints/BP_Cube_Child.BP_Cube_Child_C" (`KismetMathLibrary.MakeTransform` (`KismetMathLibrary.MakeVector` (+ _returnvalue_x (`KismetMathLibrary.Conv_IntToDouble` (* _index (`self.Padding`)))) (+ _returnvalue_y (`KismetMathLibrary.Conv_IntToDouble` (* _index_2 (`self.Padding`)))) _returnvalue_z)) "Undefined" "MultiplyWithRoot" null null))
      (`KismetArrayLibrary.Array_Add` (`self.CubesArray`) _returnvalue))))

(fn `GetCubesForWin`
  (returns (AmountCubes :type Integer))
  (return (`KismetArrayLibrary.Array_Length` (`self.CubesArray`))))

(fn `UserConstructionScript`
  (for _index (range 1 (+ (`self.X`) 1))
    (for _index_2 (range 1 (+ (`self.Y`) 1))
      (bind _returnvalue (`AddComponent|NODE_AddStaticMeshComponent-0` :`RelativeTransform` (`KismetMathLibrary.MakeTransform` (`KismetMathLibrary.MakeVector` (`KismetMathLibrary.Conv_IntToDouble` (* _index (`self.Padding`))) (`KismetMathLibrary.Conv_IntToDouble` (* _index_2 (`self.Padding`)))))))
      (`KismetArrayLibrary.Array_Add` (`self.PreviewArray`) _returnvalue))))