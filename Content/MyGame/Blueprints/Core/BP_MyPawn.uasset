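; Player pawn that spawns balls and tracks the player's lives.
; SpawnBall creates a BP_Ball at the Arrow component's location, only while lives remain and no ball is alive.
; It binds to the ball's destroyed event, which costs a life and prints a Russian game-over message when none are left.
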(event `SpawnBall`
  (if (not (<= (`self.PlayerLives`) 0))
    (`self.AliveBall`
      (:`then`)
      (:`else`
        (bind _returnvalue (`|SpawnActorFromClass` "/Game/MyGame/Blueprints/BP_Ball.BP_Ball_C" (`KismetMathLibrary.MakeTransform` (`SceneComponent.K2_GetComponentLocation` (`self.Arrow`))) "Undefined" "MultiplyWithRoot" null null))
        (bind _output_get (set `self.AliveBall` _returnvalue))
        (add `self.OnDestroyed` _output_get (delegate `BallIsDead`))))))

(event `BallIsDead` :!signature `self.OnDestroyed`
  (params (DestroyedActor :type "Actor Object Reference"))
  (bind _result (`/Engine/EditorBlueprintResources/StandardMacros.DecrementInt` (`self.PlayerLives`))
    (:`  `
      (if (<= _result 0)
        (`KismetSystemLibrary.PrintString` "Игра окончена")))))

(fn `UserConstructionScript`)