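; BP_Ball is a ball actor that moves itself and bounces off whatever it hits.
; Each tick it sweeps its Sphere component along Direction scaled by Speed and delta time, using only X and Y.
; On a blocking hit it reflects Direction around the surface normal and raises Speed by AddedSpeed up to a fixed cap, so movement needs no physics simulation.
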(event `self.ReceiveTick`
  (params (DeltaSeconds :type "Float (single-precision)"))
  (bind (_returnvalue_x _returnvalue_y) (`KismetMathLibrary.BreakVector` (* (`self.Direction`) (* DeltaSeconds (`self.Speed`)))))
  (bind _sweephitresult (`SceneComponent.K2_AddWorldOffset` (`self.Sphere`) (`KismetMathLibrary.MakeVector` _returnvalue_x _returnvalue_y) true false))
  (bind (_bblockinghit _binitialoverlap _time _distance _location _impactpoint _normal) (`GameplayStatics.BreakHitResult` _sweephitresult))
  (if _bblockinghit
    (set `self.Direction` (`KismetMathLibrary.GetReflectionVector` (`self.Direction`) _normal))
    (set `self.Speed` (`KismetMathLibrary.FMin` (+ (`self.Speed`) (`self.AddedSpeed`)) 4000.0))))

(fn `UserConstructionScript`)